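; Trigger volume that confuses the player by shifting the ThirdPersonCharacter's MouseInvert value, likely inverting mouse control.
; On overlap begin it plays a 2D confusion sound and subtracts a fixed amount from MouseInvert.
; On overlap end it waits a few seconds, then adds the same amount back, so the effect lingers after leaving.
; The change is relative rather than an absolute set.
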(event `self.CollisionComponent.OnComponentBeginOverlap`
  (params (OverlappedComponent :type "PrimitiveComponent Object Reference") (OtherActor :type "Actor Object Reference") (OtherComp :type "PrimitiveComponent Object Reference") (OtherBodyIndex :type Integer) (bFromSweep :type Boolean) (SweepResult :type "HitResult Structure (by ref)"))
  (bind _asthird_person_character (cast `/Game/Character_ThirdPerson/ThirdPersonBP/Blueprints/ThirdPersonCharacter` OtherActor))
  (`GameplayStatics.PlaySound2D` "/Game/Music/Confusion_-_SOUND_EFFECT_-_Verwirrung_SOUNDS__mp3cut_net_.Confusion_-_SOUND_EFFECT_-_Verwirrung_SOUNDS__mp3cut_net_" 1.0 1.0 0.0 null null)
  (set `/Game/Character_ThirdPerson/ThirdPersonBP/Blueprints/ThirdPersonCharacter.MouseInvert` (- (`/Game/Character_ThirdPerson/ThirdPersonBP/Blueprints/ThirdPersonCharacter.MouseInvert` _asthird_person_character) 2.0) _asthird_person_character))

(event `self.CollisionComponent.OnComponentEndOverlap`
  (params (OverlappedComponent :type "PrimitiveComponent Object Reference") (OtherActor :type "Actor Object Reference") (OtherComp :type "PrimitiveComponent Object Reference") (OtherBodyIndex :type Integer))
  (bind _asthird_person_character (cast `/Game/Character_ThirdPerson/ThirdPersonBP/Blueprints/ThirdPersonCharacter` OtherActor))
  (`KismetSystemLibrary.Delay` 5.0)
  (set `/Game/Character_ThirdPerson/ThirdPersonBP/Blueprints/ThirdPersonCharacter.MouseInvert` (+ (`/Game/Character_ThirdPerson/ThirdPersonBP/Blueprints/ThirdPersonCharacter.MouseInvert` _asthird_person_character) 2.0) _asthird_person_character))

(fn `UserConstructionScript`)