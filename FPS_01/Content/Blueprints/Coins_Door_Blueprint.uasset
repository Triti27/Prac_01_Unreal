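; Coin-gated door Blueprint that opens when the player reaches it holding exactly three coins.
; BeginPlay caches the door mesh's world position and the EndLocation component's position as start and end points.
; When a ThirdPersonCharacter overlaps PlayerTouch, it checks the truncated coin count, plays a door sound and runs a timeline that lerps the mesh to the end position without sweep.
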(event `self.ReceiveBeginPlay`
  ;[1 1 1] Change Location Door
  (set `self.StartPos` (`SceneComponent.K2_GetComponentLocation` (`self.StaticMeshComponent`)))
  (set `self.EndPos` (`SceneComponent.K2_GetComponentLocation` (`self.EndLocation`))))

(event `self.PlayerTouch.OnComponentBeginOverlap`
  (params (OverlappedComponent :type "PrimitiveComponent Object Reference") (OtherActor :type "Actor Object Reference") (OtherComp :type "PrimitiveComponent Object Reference") (OtherBodyIndex :type Integer) (bFromSweep :type Boolean) (SweepResult :type "HitResult Structure (by ref)"))
  ;[1 1 1] Detect Collision and Num of coins
  (bind _asthird_person_character (cast `/Game/Character_ThirdPerson/ThirdPersonBP/Blueprints/ThirdPersonCharacter` OtherActor))
  (if (== OtherActor _asthird_person_character)
    (if (== (`KismetMathLibrary.FTrunc` (`/Game/Character_ThirdPerson/ThirdPersonBP/Blueprints/ThirdPersonCharacter.PNumOfCoins` _asthird_person_character)) 3)
      (`GameplayStatics.PlaySound2D` "/Game/Music/Castle_door_openingclosing_sound__mp3cut_net_.Castle_door_openingclosing_sound__mp3cut_net_" 1.0 1.0 0.0 null null)
      (bind (_direction _newtrack_0) (`Timeline|Timeline_0`)
        (:`Update`
          (`SceneComponent.K2_SetWorldLocation` (`self.StaticMeshComponent`) (`KismetMathLibrary.VLerp` (`self.StartPos`) (`self.EndPos`) _newtrack_0) false false))))))

(fn `UserConstructionScript`)