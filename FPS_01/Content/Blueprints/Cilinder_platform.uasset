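; Cylinder platform actor that moves toward an end point when the player character touches it.
; BeginPlay caches the world locations of the Cylinder and the EndPos marker as start and end points.
; Overlap of PlayerTouch by a ThirdPersonCharacter plays a timeline that lerps the cylinder between them without sweep, with no reverse or reset logic.
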(event `self.ReceiveBeginPlay`
  (set `self.StartLock` (`SceneComponent.K2_GetComponentLocation` (`self.Cylinder`)))
  (set `self.EndLock` (`SceneComponent.K2_GetComponentLocation` (`self.EndPos`))))

(event `self.PlayerTouch.OnComponentBeginOverlap`
  (params (OverlappedComponent :type "PrimitiveComponent Object Reference") (OtherActor :type "Actor Object Reference") (OtherComp :type "PrimitiveComponent Object Reference") (OtherBodyIndex :type Integer) (bFromSweep :type Boolean) (SweepResult :type "HitResult Structure (by ref)"))
  (cast `/Game/Character_ThirdPerson/ThirdPersonBP/Blueprints/ThirdPersonCharacter` OtherActor)
  (bind (_direction _newtrack_0) (`Timeline|Timeline_0`)
    (:`Update`
      (`SceneComponent.K2_SetWorldLocation` (`self.Cylinder`) (`KismetMathLibrary.VLerp` (`self.StartLock`) (`self.EndLock`) _newtrack_0) false false))))

(fn `UserConstructionScript`)