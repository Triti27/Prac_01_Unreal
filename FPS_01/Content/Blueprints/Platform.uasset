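; Platform Blueprint that moves from its starting spot to a target position when the player steps into its trigger.
; On BeginPlay it caches the world locations of the platform and the EndPosition component.
; An overlap of PlayerTouch by the ThirdPersonCharacter plays the Move timeline, which lerps the platform's world location between those points without sweeping.
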(event `self.ReceiveBeginPlay`
  (set `self.Start_location` (`SceneComponent.K2_GetComponentLocation` (`self.Plataform`)))
  (set `self.End_location` (`SceneComponent.K2_GetComponentLocation` (`self.EndPosition`))))

(event `self.PlayerTouch.OnComponentBeginOverlap`
  (params (OverlappedComponent :type "PrimitiveComponent Object Reference") (OtherActor :type "Actor Object Reference") (OtherComp :type "PrimitiveComponent Object Reference") (OtherBodyIndex :type Integer) (bFromSweep :type Boolean) (SweepResult :type "HitResult Structure (by ref)"))
  (cast `/Game/Character_ThirdPerson/ThirdPersonBP/Blueprints/ThirdPersonCharacter` OtherActor)
  (bind (_direction _newtrack_0) (`Timeline|Move`)
    (:`Update`
      (`SceneComponent.K2_SetWorldLocation` (`self.Plataform`) (`KismetMathLibrary.VLerp` (`self.Start_location`) (`self.End_location`) _newtrack_0) false false))))

(fn `UserConstructionScript`)