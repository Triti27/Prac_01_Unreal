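; Key is a collectible pickup actor that adds to the player's key count.
; Tick spins the Cylinder mesh by adding a fixed roll each frame, so the speed depends on frame rate.
; When a ThirdPersonCharacter overlaps the Box, it plays a 2D lock sound, increments the character's PNumOfKeys, then destroys itself after a short delay.
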(event `self.ReceiveTick`
  (params (DeltaSeconds :type "Float (single-precision)"))
  (bind _cylinder (`self.Cylinder`))
  (bind (_relativerotation_roll _relativerotation_pitch _relativerotation_yaw) (`KismetMathLibrary.BreakRotator` (`SceneComponent.RelativeRotation` _cylinder)))
  ;[1 1 1] Rotate
  (`SceneComponent.K2_SetRelativeRotation` _cylinder (`KismetMathLibrary.MakeRotator` (+ _relativerotation_roll 1.0) _relativerotation_pitch _relativerotation_yaw) false false))

(event `self.Box.OnComponentBeginOverlap`
  (params (OverlappedComponent :type "PrimitiveComponent Object Reference") (OtherActor :type "Actor Object Reference") (OtherComp :type "PrimitiveComponent Object Reference") (OtherBodyIndex :type Integer) (bFromSweep :type Boolean) (SweepResult :type "HitResult Structure (by ref)"))
  ;[1 1 1] Detect and destroy with collison
  (bind _asthird_person_character (cast `/Game/Character_ThirdPerson/ThirdPersonBP/Blueprints/ThirdPersonCharacter` OtherActor))
  (`GameplayStatics.PlaySound2D` "/Game/Music/Door_Close_and_Lock_Sound_Effect__mp3cut_net_.Door_Close_and_Lock_Sound_Effect__mp3cut_net_" 1.0 1.0 0.0 null null)
  (set `/Game/Character_ThirdPerson/ThirdPersonBP/Blueprints/ThirdPersonCharacter.PNumOfKeys` (+ (`/Game/Character_ThirdPerson/ThirdPersonBP/Blueprints/ThirdPersonCharacter.PNumOfKeys` _asthird_person_character) 1) _asthird_person_character)
  (`KismetSystemLibrary.Delay` 0.1)
  (`self.K2_DestroyActor`))

(fn `UserConstructionScript`)