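; DistanceDoor is a door actor that slides open when the third-person character enters its trigger volume and closes when they leave.
; On BeginPlay it caches the Door's world position and the EndLock component's position as the two endpoints.
; PlayerTouch overlap begin and end play or reverse the Move timeline, which lerps the Door's location between those endpoints.
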(event `self.ReceiveBeginPlay`
  (set `self.StartLock` (`SceneComponent.K2_GetComponentLocation` (`self.Door`)))
  (set `self.EndLoc` (`SceneComponent.K2_GetComponentLocation` (`self.EndLock`))))

(event `self.PlayerTouch.OnComponentBeginOverlap`
  (params (OverlappedComponent :type "PrimitiveComponent Object Reference") (OtherActor :type "Actor Object Reference") (OtherComp :type "PrimitiveComponent Object Reference") (OtherBodyIndex :type Integer) (bFromSweep :type Boolean) (SweepResult :type "HitResult Structure (by ref)"))
  (cast `/Game/Character_ThirdPerson/ThirdPersonBP/Blueprints/ThirdPersonCharacter` OtherActor)
  (bind (_direction _newtrack_0) (`Timeline|Move` :!label _label)
    (:`Update`
      (`SceneComponent.K2_SetWorldLocation` (`self.Door`) (`KismetMathLibrary.VLerp` (`self.StartLock`) (`self.EndLoc`) _newtrack_0) false false))))

(event `self.PlayerTouch.OnComponentEndOverlap`
  (params (OverlappedComponent :type "PrimitiveComponent Object Reference") (OtherActor :type "Actor Object Reference") (OtherComp :type "PrimitiveComponent Object Reference") (OtherBodyIndex :type Integer))
  (cast `/Game/Character_ThirdPerson/ThirdPersonBP/Blueprints/ThirdPersonCharacter` OtherActor)
  (goto _label :!via `Reverse`))

(fn `UserConstructionScript`)