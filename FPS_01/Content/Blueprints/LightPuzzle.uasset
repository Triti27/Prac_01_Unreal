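; Light puzzle Blueprint that tracks how many lights count toward solving the puzzle and moves a cube when all are counted.
; AddTO increments a counter and compares it to the number of Light actors in the level, firing WinningCondition on a match, while RemoveFrom decrements it without going below zero.
; WinningCondition plays a timeline whose track adds a relative Z offset to the cube on each update.
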(event `AddTO`
  ;[1 1 1] Add until int = amount of lights in the scene
  (set `self.Int` (+ (`self.Int`) 1))
  (bind _outactors (`GameplayStatics.GetAllActorsOfClass` "/Game/Blueprints/Light.Light_C"))
  (if (== (`KismetArrayLibrary.Array_Length` _outactors) (`self.Int`))
    (`self.WinningCondition`)))

(event `RemoveFrom`
  (bind _int (`self.Int`))
  ;[1 1 1] TakeAwayInt
  (if (> _int 0)
    (set `self.Int` (- _int 1))))

(event `WinningCondition`
  ;[1 1 1] Winnning Condition
  (bind (_direction _newtrack_0) (`Timeline|WinnerWinner`)
    (:`Update`
      (`SceneComponent.K2_AddRelativeLocation` (`self.Cube`) (`KismetMathLibrary.MakeVector` 0.0 0.0 _newtrack_0) false false))))

(event `self.ReceiveTick`
  (params (DeltaSeconds :type "Float (single-precision)"))
  ;[1 1 1] Informer
)

(fn `UserConstructionScript`)